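; BP_ZombieTest is a test zombie enemy that chases the player and self-destructs 60 seconds after spawning.
; PawnSensing sets a seen flag and starts an AI MoveTo toward the player pawn.
; Capsule overlap with the tow truck, either civil car or a bullet kills it through shared logic.
; Death disables capsule collision, hides the spotlight, ragdolls the mesh and adds a Niagara effect, then destroys the actor after a delay.
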(event `self.ReceiveBeginPlay`
  (`KismetSystemLibrary.Delay` 60.0)
  (`self.K2_DestroyActor`))

(event `self.CapsuleComponent.OnComponentBeginOverlap`
  (params (OverlappedComponent :type "PrimitiveComponent Object Reference") (OtherActor :type "Actor Object Reference") (OtherComp :type "PrimitiveComponent Object Reference") (OtherBodyIndex :type Integer) (bFromSweep :type Boolean) (SweepResult :type "HitResult Structure (by ref)"))
  (`|ExecutionSequence`
    (:`then_0`
      (cast `/Game/VehicleTemplate/Blueprints/TowTruck_Pawn` OtherActor))
    (:`then_1`
      (cast `/Game/VehicleTemplate/Blueprints/CivilCarBP/BP_CivilCar` OtherActor))
    (:`then_2`
      (cast `/Game/Turret/BP_Bullet` OtherActor))
    (:`then_3`
      (cast `/Game/VehicleTemplate/Blueprints/CivilCarBP/BP_CivilCar_2` OtherActor)))
  (`PrimitiveComponent.SetCollisionEnabled` (`self.CapsuleComponent`) "NoCollision")
  (`SceneComponent.SetVisibility` (`self.SpotLight`) false false)
  (`PrimitiveComponent.SetSimulatePhysics` (`self.Mesh`) true)
  (`AddComponent|NODE_AddNiagaraComponent-1`)
  (`KismetSystemLibrary.Delay` 5.0)
  (`MovementComponent.StopMovementImmediately` (`self.CharacterMovement`))
  (`self.K2_DestroyActor`))

(event `self.PawnSensing.OnSeePawn`
  (params (Pawn :type "Pawn Object Reference"))
  (set `self.IsSeeingPlayer` true)
  (`self.Follow Player`))

(event `Follow Player`
  (if (`self.IsSeeingPlayer`)
    (`|AIMoveTo` self (0.0 0.0 0.0) (`GameplayStatics.GetPlayerPawn` 0) 5.0 true)))

(fn `UserConstructionScript`)