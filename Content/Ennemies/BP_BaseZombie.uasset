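; Base zombie enemy that reacts to sighting pawns and dies when its hit box is overlapped.
; PawnSensing sets a seeing flag, never cleared here, and calls FollowPlayer, whose AIMoveTo takes the player character as both moved pawn and target, rather than moving the zombie itself.
; Any HitBox overlap turns on collision and physics for Z, adds a Niagara effect, then destroys the actor after a short delay.
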(event `self.HitBox.OnComponentBeginOverlap`
  (params (OverlappedComponent :type "PrimitiveComponent Object Reference") (OtherActor :type "Actor Object Reference") (OtherComp :type "PrimitiveComponent Object Reference") (OtherBodyIndex :type Integer) (bFromSweep :type Boolean) (SweepResult :type "HitResult Structure (by ref)"))
  (`PrimitiveComponent.SetCollisionEnabled` (`self.Z`) "QueryAndPhysics")
  (`PrimitiveComponent.SetSimulatePhysics` (`self.Z`) true)
  (`AddComponent|NODE_AddNiagaraComponent-0`)
  (`KismetSystemLibrary.Delay` 3.0)
  (`self.K2_DestroyActor`))

(event `self.PawnSensing.OnSeePawn`
  (params (Pawn :type "Pawn Object Reference"))
  (set `self.IsSeeingPlayer` true)
  (`self.Follow Player`))

(event `Follow Player`
  (bind _returnvalue (`GameplayStatics.GetPlayerCharacter` 0))
  (if (`self.IsSeeingPlayer`)
    (`|AIMoveTo` _returnvalue (0.0 0.0 0.0) _returnvalue)))

(fn `UserConstructionScript`)