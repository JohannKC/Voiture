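; BP_Chain is a procedural physics chain actor that spans a configurable number of segments between its Start and End components.
; The construction script spawns static mesh links and physics constraints, swapping the first link for Start and appending End.
; Each constraint joins neighboring links, stacked along Z with alternating 90-degree yaw to form interlocked links, and End moves to the last constraint.
; The event graph has no active logic.
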(fn `UserConstructionScript`
  (bind _physicsconstraints (`self.PhysicsConstraints`))
  (bind _chainsegments (`self.ChainSegments`))
  (bind _chainsegments_2 (`self.ChainSegments`))
  (bind _chainsegments_3 (`self.ChainSegments`))
  (for _ (range (+ (`self.Segment Number`) 1))
    (bind _returnvalue (`AddComponent|NODE_AddStaticMeshComponent-0` :`RelativeTransform` (`KismetMathLibrary.MakeTransform` (0.0 0.0 0.0) (struct) (5.0 5.0 5.0))))
    (`KismetArrayLibrary.Array_AddUnique` (`self.ChainSegments`) _returnvalue)
    (bind _returnvalue_2 (`AddComponent|NODE_AddPhysicsConstraintComponent-0`))
    (`KismetArrayLibrary.Array_AddUnique` (`self.PhysicsConstraints`) _returnvalue_2))
  (`ActorComponent.K2_DestroyComponent` (`|GetArrayItem` _chainsegments))
  (`KismetArrayLibrary.Array_Remove` _chainsegments)
  (`KismetArrayLibrary.Array_Insert` _chainsegments_2 (`self.start`))
  (`KismetArrayLibrary.Array_Insert` _chainsegments_2 (`self.end`) (+ (`KismetArrayLibrary.Array_LastIndex` _chainsegments_2) 1))
  (for (_array_element _array_index) (`self.PhysicsConstraints`)
    (bind _output (`|GetArrayItem` _chainsegments_3 _array_index))
    (`PhysicsConstraintComponent.SetConstrainedComponents` _array_element _output "None" (`|GetArrayItem` _chainsegments_3 (+ _array_index 1)) "None")
    (bind _returnvalue_3 (`KismetMathLibrary.SelectFloat` 0.0 90.0 (== (mod _array_index 2) 0)))
    (`SceneComponent.K2_SetRelativeLocationAndRotation` _output (`KismetMathLibrary.MakeVector` 0.0 0.0 (`KismetMathLibrary.Conv_IntToDouble` (+ (* _array_index 17) 17))) (`KismetMathLibrary.MakeRotator` 0.0 90.0 _returnvalue_3) false false)
    (`SceneComponent.K2_SetRelativeLocationAndRotation` _array_element (`KismetMathLibrary.MakeVector` 0.0 0.0 (`KismetMathLibrary.Conv_IntToDouble` (+ (* _array_index 17) 22))) (`KismetMathLibrary.MakeRotator` 0.0 0.0 _returnvalue_3) false false))
  (`SceneComponent.K2_SetRelativeLocation` (`self.end`) (`SceneComponent.RelativeLocation` (`|GetArrayItem` _physicsconstraints (`KismetArrayLibrary.Array_LastIndex` _physicsconstraints))) false false))